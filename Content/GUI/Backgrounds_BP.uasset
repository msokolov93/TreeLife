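; Backgrounds actor that manages a sequence of horizontally scrolling Paper2D backdrops.
; On BeginPlay it gathers sprite actors tagged "Background", then positions and shows the first two as an active/next pair.
; MoveBackgrounds steps the pair along negative X, advancing the array index and re-initializing when the next sprite hits an exact X threshold.
; Nothing in this graph drives MoveBackgrounds; Tick is disabled.
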(event `self.ReceiveBeginPlay`
  (`self.GetArrayOfBackgrounds`)
  (`self.InitBackgrounds`)
  (`KismetSystemLibrary.PrintString` "Init Successful" true true (struct :`R` 1.0 :`G` 0.869393 :`A` 1.0) 10.0))

(fn `GetArrayOfBackgrounds`
  (bind _outactors (`GameplayStatics.GetAllActorsOfClassWithTag` "/Script/Paper2D.PaperSpriteActor" "Background"))
  (bind _output_get (set `self.ArrayBackgrounds` _outactors))
  (`KismetSystemLibrary.PrintString` (`KismetStringLibrary.Concat_StrStr` "Array count = " (`KismetStringLibrary.Conv_IntToString` (`KismetArrayLibrary.Array_Length` _output_get)))))

(fn `HideActiveBackground`
  (`SceneComponent.SetVisibility` (`Actor.RootComponent` (`self.ActiveBackground`)) false false))

(fn `InitBackgrounds`
  (`self.SetActiveBackground`)
  (`self.SetBackgroundStartLocation`)
  (`self.SetBackgroundsVisibile`))

(fn `Move_Backgrounds`
  (if (and (== -1080.0 (.x (`self.K2_GetActorLocation` (`self.ActiveBackground`)))) (== (+ (`self.ActiveCounter`) 1) (`KismetArrayLibrary.Array_Length` (`self.ArrayBackgrounds`))))
    (return)
    (else
      (`self.MoveOnce` (`self.ActiveBackground`))
      (`self.MoveOnce` (`self.NextBackground`))
      (if (== 1080.0 (.x (`self.K2_GetActorLocation` (`self.NextBackground`))))
        (`/Engine/EditorBlueprintResources/StandardMacros.IncrementInt` (`self.ActiveCounter`)
          (:`  `
            (`self.HideActiveBackground`)
            (`self.InitBackgrounds`)))
        (else
          (return))))))

(fn `MoveOnce`
  (params (Target :type "Actor Object Reference"))
  (`self.K2_SetActorLocation` Target (+ (`self.K2_GetActorLocation` Target) (-108.0 0.0 0.0)) false false))

(fn `SetActiveBackground`
  (locals (BackgroundTag :type Name))
  (bind _activecounter (`self.ActiveCounter`))
  (bind _arraybackgrounds (`self.ArrayBackgrounds`))
  (set `self.ActiveBackground` (`|GetArrayItem` _arraybackgrounds _activecounter))
  (set `self.NextBackground` (`|GetArrayItem` _arraybackgrounds (+ _activecounter 1))))

(fn `SetBackgroundStartLocation`
  (locals (StartLocationActive :type "Vector Structure" :default (1080.0 -430.0 870.0)) (StartLocationNext :type "Vector Structure" :default (4320.0 -430.0 870.0)))
  (`self.K2_SetActorLocation` (`self.ActiveBackground`) (`local.StartLocationActive`) false false)
  (`self.K2_SetActorLocation` (`self.NextBackground`) (`local.StartLocationNext`) false false))

(fn `SetBackgroundsVisibile`
  (`SceneComponent.SetVisibility` (`Actor.RootComponent` (`self.ActiveBackground`)) true true)
  (`SceneComponent.SetVisibility` (`Actor.RootComponent` (`self.NextBackground`)) true true))

(fn `UserConstructionScript`)