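; Player tree character for a click-driven growing game, broadcasting left clicks and a one-second game tick.
; The tick swaps the flipbook by TreeLevel and randomly applies scaled weather damage to HP in the GameInstance.
; A self-rescheduling random timer rolls tiered weather, with harsher tiers possible only from level 6.
; Parallel arrays supply each weather's name, texture, damage, light and water, which are published to the GameInstance.
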(event `Key|LeftMouseButton`
  (params (Key :type "Key Structure"))
  (:`Pressed`
    (`self.OnClick`)))

(event `self.ReceiveBeginPlay`
  (`self.GenerateWeather` false)
  (`PaperFlipbookComponent.SetFlipbook` (`self.Sprite`) "/Game/TreeLife/Sprites/Irrelevant/old_tree_sprites/tree_lvl_1.tree_lvl_1")
  (`KismetSystemLibrary.K2_SetTimer` null "UpdateWorld" 1.0 true)
  (`KismetSystemLibrary.K2_SetTimer` null "UpdateWeather" 0.1))

(event `UpdateWorld`
  (`self.UpdateTreeSprites`)
  (`self.DealDamage`)
  (`self.OnGameTick`))

(event `UpdateWeather`
  (`KismetSystemLibrary.K2_SetTimer` null "UpdateWeather" (`KismetMathLibrary.RandomFloatInRange` 10.0 20.0))
  (`self.GenerateWeather` false))

(event `self.ReceiveTick`
  (params (DeltaSeconds :type "Float (single-precision)"))
  (set `PlayerController.bShowMouseCursor` true (`GameplayStatics.GetPlayerController` 0)))

(fn `DealDamage`
  (bind _asgame_instance (cast `/Game/GlobalBlueprints/GameInstance` (`GameplayStatics.GetGameInstance`)))
  (if (`KismetMathLibrary.RandomBool`)
    (bind _asgame_instance_2 (cast `/Game/GlobalBlueprints/GameInstance` (`GameplayStatics.GetGameInstance`)))
    (bind _asgame_instance_3 (cast `/Game/GlobalBlueprints/GameInstance` (`GameplayStatics.GetGameInstance`)))
    (bind _returnvalue (* (`/Game/GlobalBlueprints/GameInstance.WeatherDamageGlobal` _asgame_instance) (`KismetMathLibrary.RandomFloat`)))
    (set `/Game/GlobalBlueprints/GameInstance.HP` (`KismetMathLibrary.FMax` 0.0 (- (`/Game/GlobalBlueprints/GameInstance.HP` _asgame_instance_2) _returnvalue)) _asgame_instance_3)
    (`KismetSystemLibrary.PrintString` (`KismetStringLibrary.Concat_StrStr` "Deamage Inflicted = " (`KismetStringLibrary.Conv_DoubleToString` _returnvalue)) false true (struct :`R` 1.0 :`B` 0.042226 :`A` 1.0) 10.0)
    (return)
    (else
      (`KismetSystemLibrary.PrintString` "Damage Avoided" false true (struct :`G` 1.0 :`B` 0.486301 :`A` 1.0)))))

(fn `GenerateWeather`
  (params (IsDebug :type Boolean :default false) (ValueDebug :type Integer))
  (locals (WeatherSeed :type Integer) (WeatherArray :type "Array of String") (WeatherTextureArray :type "Array of Texture Object Reference") (ReturnedWeatherRoll :type Integer) (WeatherLightArray :type "Array of Float (double-precision)") (WeatherWaterArray :type "Array of Float (double-precision)") (WeatherDamageValue :type "Array of Float (double-precision)"))
  (set `local.WeatherSeed` (`KismetMathLibrary.RandomIntegerInRange` 0 9))
  ;[1 1 1] Special Events Weather manipulation
  (bind _asgame_instance (cast `/Game/GlobalBlueprints/GameInstance` (`GameplayStatics.GetGameInstance`)))
  (if (< (`/Game/GlobalBlueprints/GameInstance.Tree_Level` _asgame_instance) 6)
    (set `local.WeatherSeed` (`KismetMathLibrary.RandomIntegerInRange` 0 5)))
  (switch `int` (`local.WeatherSeed`)
    (:`0`
      ;[1 1 1] Good
      (`/Engine/EditorBlueprintResources/StandardMacros.DoOnce` false :!label _label
        (:`Completed`
          (set `local.ReturnedWeatherRoll` (`KismetMathLibrary.RandomIntegerInRange` 0 3)))))
    (:`1`
      (goto _label))
    (:`2`
      (goto _label))
    (:`3`
      (goto _label))
    (:`4`
      (goto _label))
    (:`5`
      (goto _label))
    (:`6`
      ;[1 1 1] Medium
      (`/Engine/EditorBlueprintResources/StandardMacros.DoOnce` false :!label _label_2
        (:`Completed`
          (set `local.ReturnedWeatherRoll` (`KismetMathLibrary.RandomIntegerInRange` 4 7)))))
    (:`7`
      (goto _label_2))
    (:`8`
      (goto _label_2))
    (:`9`
      ;[1 1 1] Bad
      (`/Engine/EditorBlueprintResources/StandardMacros.DoOnce` false
        (:`Completed`
          (set `local.ReturnedWeatherRoll` (`KismetMathLibrary.RandomIntegerInRange` 8 11))))))
  (if (`local.IsDebug`)
    (set `local.ReturnedWeatherRoll` (`local.ValueDebug`)))
  ;[1 1 1] Weather Name Table, Weather Texture table, Debugg string
  (`KismetSystemLibrary.PrintString` "Hello" false false (struct :`R` 1.0 :`G` 0.03805 :`B` 0.321026 :`A` 1.0) 100.0)
  (set `self.Weather` (`|GetArrayItem` (`local.WeatherArray`) (`local.ReturnedWeatherRoll`)))
  (set `self.WeatherTexture` (`|GetArrayItem` (`local.WeatherTextureArray`) (`local.ReturnedWeatherRoll`)))
  (set `self.WeatherDamage` (`|GetArrayItem` (`local.WeatherDamageValue`) (`local.ReturnedWeatherRoll`)))
  (`KismetSystemLibrary.PrintString` (`KismetStringLibrary.Concat_StrStr` " Weather seed = " (`KismetStringLibrary.Conv_IntToString` (`local.WeatherSeed`)) " Weather = " (`self.Weather`) " Weather texture = " (`KismetSystemLibrary.GetDisplayName` (`self.WeatherTexture`))) false true (struct :`R` 1.0 :`G` 0.03805 :`B` 0.321026 :`A` 1.0) 100.0)
  ;[1 1 1] Cast Name, Texture to Game Instance
  (bind _asgame_instance_2 (cast `/Game/GlobalBlueprints/GameInstance` (`GameplayStatics.GetGameInstance`)))
  (set `/Game/GlobalBlueprints/GameInstance.WeatherTextureGlobal` (`self.WeatherTexture`) _asgame_instance_2)
  (set `/Game/GlobalBlueprints/GameInstance.WeatherNameGlobal` (`self.Weather`) _asgame_instance_2)
  (set `/Game/GlobalBlueprints/GameInstance.WeatherDamageGlobal` (`self.WeatherDamage`) _asgame_instance_2)
  ;[1 1 1] Get Light, Water from Weather, Cast to Game Instance
  (set `self.WeatherLight` (`|GetArrayItem` (`local.WeatherLightArray`) (`local.ReturnedWeatherRoll`)))
  (set `self.WeatherWater` (`|GetArrayItem` (`local.WeatherWaterArray`) (`local.ReturnedWeatherRoll`)))
  (bind _asgame_instance_3 (cast `/Game/GlobalBlueprints/GameInstance` (`GameplayStatics.GetGameInstance`)))
  (set `/Game/GlobalBlueprints/GameInstance.WeatherLightGlobal` (`self.WeatherLight`) _asgame_instance_3)
  (set `/Game/GlobalBlueprints/GameInstance.WeatherWaterGlobal` (`self.WeatherWater`) _asgame_instance_3)
  ;[1 1 1] Debug Light and Water
  (`KismetSystemLibrary.PrintString` (`KismetStringLibrary.Concat_StrStr` " Weather = " (`self.Weather`) " Weather Light = " (`KismetStringLibrary.Conv_DoubleToString` (`self.WeatherLight`)) " Weather Water = " (`KismetStringLibrary.Conv_DoubleToString` (`self.WeatherWater`))) false true (struct :`R` 1.0 :`G` 0.451592 :`A` 1.0) 100.0)
  (return))

(fn `UpdateBackgroundPosition`)

(fn `UpdateLevel`
  (locals (local_Clicks :type "Float (double-precision)") (local_Level_Points :type "Float (double-precision)") (local_Level :type "Float (double-precision)")))

(fn `UpdateTreeSprites`
  (locals (local_Level :type "Float (double-precision)"))
  (bind _asgame_instance (cast `/Game/GlobalBlueprints/GameInstance` (`GameplayStatics.GetGameInstance`)))
  (bind _output_get (set `local.local_Level` (`KismetMathLibrary.Conv_IntToDouble` (`/Game/GlobalBlueprints/GameInstance.Tree_Level` _asgame_instance))))
  (`/Engine/EditorBlueprintResources/StandardMacros.CompareFloat` _output_get (`self.Level_4_Sprite`)
    (:`>`
      (`PaperFlipbookComponent.SetFlipbook` (`self.Sprite`) "/Game/TreeLife/Sprites/Irrelevant/old_tree_sprites/tree_lvl_4.tree_lvl_4" :!label _label))
    (:`==`
      (goto _label))
    (:`<`
      (`/Engine/EditorBlueprintResources/StandardMacros.CompareFloat` (`local.local_Level`) (`self.Level_3_Sprite`)
        (:`>`
          (`PaperFlipbookComponent.SetFlipbook` (`self.Sprite`) "/Game/TreeLife/Sprites/Irrelevant/old_tree_sprites/tree_lvl_3.tree_lvl_3" :!label _label_2))
        (:`==`
          (goto _label_2))
        (:`<`
          (`/Engine/EditorBlueprintResources/StandardMacros.CompareFloat` (`local.local_Level`) (`self.Level_2_Sprite`)
            (:`>`
              (`PaperFlipbookComponent.SetFlipbook` (`self.Sprite`) "/Game/TreeLife/Sprites/Irrelevant/old_tree_sprites/tree_lvl_2.tree_lvl_2" :!label _label_3))
            (:`==`
              (goto _label_3))
            (:`<`
              (`/Engine/EditorBlueprintResources/StandardMacros.CompareFloat` (`local.local_Level`) (`self.Level_1_Sprite`)
                (:`>`
                  _)
                (:`==`
                  _))
              (`PaperFlipbookComponent.SetFlipbook` (`self.Sprite`) "/Game/TreeLife/Sprites/Irrelevant/old_tree_sprites/tree_lvl_1.tree_lvl_1")))))))
  (return))

(fn `UserConstructionScript`)